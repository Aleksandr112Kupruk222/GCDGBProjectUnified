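; Player Blueprint for a timed survival level, with Enhanced Input movement, health and a HUD widget.
; A looping one-second timer counts down to the win screen, while death opens the lose screen, storing health or remaining time respectively in the game instance.
; Capsule hits and falling below a height threshold deal damage, and falls also respawn at the start.
; Enemy-tagged actor hits use DecreaseHealth, which skips the death check.
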(event OnComponentHit(CapsuleComponent)
  (params (HitComponent :type Primitive%20Component%20Object%20Reference) (OtherActor :type Actor%20Object%20Reference) (OtherComp :type Primitive%20Component%20Object%20Reference) (NormalImpulse :type Vector :default "0, 0, 0") (Hit :type Hit%20Result%20Structure%20%28by%20ref%29))
  (if (Actor|ActorHasTag OtherActor "Enemy")
    (Development|PrintString "Enemy")
    (CallFunction|DecreaseHealth 5.0)
    (elif (Actor|ActorHasTag OtherActor "PickUp")
      (Development|PrintString "PickUp")
      (elif (Components|ComponentHasTag OtherComp "EnemyComp")
        (CallFunction|DecreaseHealhCustomEvent 1e+01)
        (Actor|DestroyActor (Components|GetOwner OtherComp))))))

(event OnComponentBeginOverlap(CapsuleComponent)
  (params (OverlappedComponent :type Primitive%20Component%20Object%20Reference) (OtherActor :type Actor%20Object%20Reference) (OtherComp :type Primitive%20Component%20Object%20Reference) (OtherBodyIndex :type Integer) (bFromSweep :type Boolean) (SweepResult :type Hit%20Result%20Structure%20%28by%20ref%29))
  (Development|PrintString "Overlap"))

(event Custom|DecreaseHealhCustomEvent
  (params (Damage :type Float%20%28double-precision%29))
  (bind _output_get (Variables|Default|SetHealth (- (Variables|Default|GetHealth) Damage)))
  (Development|PrintString (Utilities|String|ToString(Float) _output_get))
  (if (< (Variables|Default|GetHealth) 0.0)
    (CallFunction|Death)))

(event Custom|Death
  (Variables|/Game/MainMenu/BP_CustomGameInstance.BP_CustomGameInstance_C|SetTimer (Variables|Default|GetGameInstanceRef) (Variables|Default|GetTimer))
  (Game|OpenLevel(byObjectReference) "/Game/MainMenu/LoseScreen.LoseScreen"))

(event Custom|PlayerFellOff
  (Transformation|SetActorLocation (Variables|Default|GetStartLocation) false false)
  (CallFunction|DecreaseHealhCustomEvent 51.0))

(event Custom|DecreaseTimer
  (bind _result (Math|Integer|DecrementInt (Variables|Default|GetTimer))
    (:%20%20
      (if (<= _result 0)
        (CallFunction|PassHealth)
        (Game|OpenLevel(byObjectReference) "/Game/MainMenu/WinScreen.WinScreen")))))

(event Custom|PassHealth
  (Variables|/Game/MainMenu/BP_CustomGameInstance.BP_CustomGameInstance_C|SetPlayerHealth (Variables|Default|GetGameInstanceRef) (Variables|Default|GetHealth)))

(event Input|EnhancedActionEvents|EnhancedInputActionIA_Move
  (params (ActionValue :type Vector%202D%20Structure) (ElapsedSeconds :type Float%20%28double-precision%29) (TriggeredSeconds :type Float%20%28double-precision%29) (InputAction :type Input%20Action%20Object%20Reference :default "/Game/Blueprints/IA_Move.IA_Move"))
  (Pawn|Input|AddMovementInput (Transformation|GetActorForwardVector) (.x ActionValue) false)
  (Pawn|Input|AddMovementInput (Transformation|GetActorRightVector) (.y ActionValue) false))

(event EventBeginPlay
  (Variables|Default|SetHealth 1e+02)
  (Variables|Default|SetStartLocation (Transformation|GetActorLocation))
  (bind _returnvalue (UserInterface|CreateWidget "/Game/Blueprints/WB_PlayerUI.WB_PlayerUI_C"))
  (Variables|Default|SetPlayerUI _returnvalue)
  (Variables|/Game/Blueprints/WB_PlayerUI.WB_PlayerUI_C|SetPlayerRef _returnvalue self)
  (UserInterface|Viewport|AddtoViewport _returnvalue 0)
  (bind _asbp_custom_game_instance (Utilities|Casting|CastToBP_CustomGameInstance (Game|GetGameInstance)))
  (Variables|Default|SetGameInstanceRef _asbp_custom_game_instance)
  (Utilities|Time|SetTimerbyEvent (delegate Custom|DecreaseTimer) 1.0 true))

(event Collision|EventActorBeginOverlap
  (params (OtherActor :type Actor%20Object%20Reference)))

(event EventTick
  (params (DeltaSeconds :type Float%20%28single-precision%29))
  (if (< (.z (Transformation|GetActorLocation)) 5e+02)
    (CallFunction|PlayerFellOff)))

(fn ConstructionScript)

(fn DecreaseHealth
  (params (Damage :type Float%20%28double-precision%29))
  (bind _output_get (Variables|Default|SetHealth (- (Variables|Default|GetHealth) Damage)))
  (Development|PrintString (Utilities|String|ToString(Float) _output_get)))